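; Player actor for a Crossy Road-style hopper that spawns as a random chicken, sheep, steer or hedgehog.
; Directional input dips and turns the actor on press, then on release moves it one step through a Timeline lerp unless a line trace is blocked.
; Car, truck or train overlap swaps in a flattened mesh, disables input through Dead, plays that animal's death sound and calls CallPlayerDeath after a delay.
; Forward presses occasionally play animal sounds.
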(event EventBeginPlay
  (bind _chicken (Variables|Default|GetChicken))
  ;[1 1 1] Set Character Model
  (bind _output_get (Variables|Default|SetIAmType (Math|Random|RandomIntegerinRange 0 3)))
  (switch int _output_get
    (:0
      (Variables|Default|SetIAmType 0))
    (:1
      (Variables|Default|SetIAmType 1)
      (Components|StaticMesh|SetStaticMesh _chicken "/Game/Meshes/whitesheep.whitesheep"))
    (:2
      (Variables|Default|SetIAmType 2)
      (Components|StaticMesh|SetStaticMesh _chicken "/Game/Meshes/steer.steer"))
    (:3
      (Variables|Default|SetIAmType 3)
      (Components|StaticMesh|SetStaticMesh _chicken "/Game/Meshes/hedgehog.hedgehog"))))

(event Collision|EventActorBeginOverlap
  (params (OtherActor :type Actor%20Object%20Reference))
  ;[1 1 1] Flatten
  (Utilities|Casting|CastTocarBP OtherActor
    (:then
      _)
    (:CastFailed
      (Utilities|Casting|CastTotruckBP OtherActor
        (:then
          _)
        (:CastFailed
          (Utilities|Casting|CastTotrainBP OtherActor)))))
  (CallFunction|SetFlattenedMesh)
  (Transformation|SetRelativeLocation (Variables|Default|GetChicken) "0.000000,0.000000,-95.000000" false false)
  (Variables|Default|Setdead true)
  (CallFunction|DeathSound)
  (Utilities|FlowControl|Delay 3.0)
  (Default|CallPlayerDeath))

(event Input|ActionEvents|InputActionplayerUp
  (params (Key :type Key%20Structure))
  (bind _returnvalue (Transformation|GetActorLocation))
  (bind _chicken (Variables|Default|GetChicken))
  (bind _returnvalue_2 (Transformation|GetWorldLocation _chicken))
  ;[1 1 1] Move Forward
  (:Pressed
    (if (not (Variables|Default|Getdead))
      (Transformation|AddActorLocalOffset "0,0.000000,-7.000000" false false)
      (Transformation|SetActorRotation "0, 0, 0")
      (CallFunction|NormalSound)))
  (:Released
    (if (not (Variables|Default|Getdead))
      (Transformation|AddActorLocalOffset "0,0.000000,7.000000" false false)
      (Variables|Default|SetstartPoint _returnvalue)
      (Variables|Default|SetendPoint (+ "35.000000, 0, 0" _returnvalue))
      (bind _returnvalue_3 (Collision|LineTraceByChannel (+ "3.000000,3.000000, 0" _returnvalue_2) (+ "35.000000,3.000000, 0" _returnvalue_2) "TraceTypeQuery1" false 0 "None"))
      (if (not _returnvalue_3)
        (bind _alpha (Timeline|MoveOverTime PlayFromStart)
          (:Update
            (Transformation|SetActorLocation (Math|Vector|Lerp(Vector) (Variables|Default|GetstartPoint) (Variables|Default|GetendPoint) _alpha) true false)))))))

(event Input|ActionEvents|InputActionplayerDown
  (params (Key :type Key%20Structure))
  (bind _defaultsceneroot (Variables|Default|GetDefaultSceneRoot))
  (bind _chicken (Variables|Default|GetChicken))
  (bind _returnvalue (Transformation|GetWorldLocation _defaultsceneroot))
  (bind _returnvalue_2 (Transformation|GetWorldLocation _chicken))
  ;[1 1 1] Move Back
  (:Pressed
    (if (not (Variables|Default|Getdead))
      (Transformation|AddActorLocalOffset "0,0.000000,-7.000000" false false)
      (Transformation|SetActorRotation "0,180.000000, 0")))
  (:Released
    (if (not (Variables|Default|Getdead))
      (Transformation|AddActorLocalOffset "0,0.000000,7.000000" false false)
      (Variables|Default|SetstartPoint _returnvalue)
      (Variables|Default|SetendPoint (+ "-35.000000,0.000000, 0" _returnvalue))
      (bind _returnvalue_3 (Collision|LineTraceByChannel (+ "0, 0, 0" _returnvalue_2) (+ "-35.000000,0.000000, 0" _returnvalue_2) "TraceTypeQuery1" false 0 "None"))
      (if (not _returnvalue_3)
        (bind _alpha (Timeline|Timeline_2 PlayFromStart)
          (:Update
            (Transformation|SetActorLocation (Math|Vector|Lerp(Vector) (Variables|Default|GetstartPoint) (Variables|Default|GetendPoint) _alpha) true false)))))))

(event Input|ActionEvents|InputActionplayerLeft
  (params (Key :type Key%20Structure))
  (bind _defaultsceneroot (Variables|Default|GetDefaultSceneRoot))
  (bind _chicken (Variables|Default|GetChicken))
  (bind _returnvalue (Transformation|GetWorldLocation _defaultsceneroot))
  (bind _returnvalue_2 (Transformation|GetWorldLocation _chicken))
  ;[1 1 1] Move Left
  (:Pressed
    (if (not (Variables|Default|Getdead))
      (Transformation|AddActorLocalOffset "0,0.000000,-7.000000" false false)
      (Transformation|SetActorRotation "0,270.000000, 0")))
  (:Released
    (if (not (Variables|Default|Getdead))
      (Transformation|AddActorLocalOffset "0,0.000000,7.000000" false false)
      (Variables|Default|SetstartPoint _returnvalue)
      (Variables|Default|SetendPoint (+ "0.000000,-35.000000, 0" _returnvalue))
      (bind _returnvalue_3 (Collision|LineTraceByChannel (+ "0, 0, 0" _returnvalue_2) (+ "0,-35.000000, 0" _returnvalue_2) "TraceTypeQuery1" false 0 "None"))
      (if (not _returnvalue_3)
        (bind _alpha (Timeline|Timeline_1 PlayFromStart)
          (:Update
            (Transformation|SetActorLocation (Math|Vector|Lerp(Vector) (Variables|Default|GetstartPoint) (Variables|Default|GetendPoint) _alpha) true false)))))))

(event Input|ActionEvents|InputActionplayerRight
  (params (Key :type Key%20Structure))
  (bind _chicken (Variables|Default|GetChicken))
  (bind _defaultsceneroot (Variables|Default|GetDefaultSceneRoot))
  (bind _returnvalue (Transformation|GetWorldLocation _chicken))
  (bind _returnvalue_2 (Transformation|GetWorldLocation _defaultsceneroot))
  ;[1 1 1] Move Right
  (:Pressed
    (if (not (Variables|Default|Getdead))
      (Transformation|AddActorLocalOffset "0,0.000000,-7.000000" false false)
      (Transformation|SetActorRotation "0,90.000000, 0")))
  (:Released
    (if (not (Variables|Default|Getdead))
      (Transformation|AddActorLocalOffset "0,0.000000,7.000000" false false)
      (Variables|Default|SetstartPoint _returnvalue_2)
      (Variables|Default|SetendPoint (+ "0.000000,35.000000, 0" _returnvalue_2))
      (bind _returnvalue_3 (Collision|LineTraceByChannel (+ "0, 0, 0" _returnvalue) (+ "0,35.000000, 0" _returnvalue) "TraceTypeQuery1" false 0 "None"))
      (if (not _returnvalue_3)
        (bind _alpha (Timeline|Timeline_0 PlayFromStart)
          (:Update
            (Transformation|SetActorLocation (Math|Vector|Lerp(Vector) (Variables|Default|GetstartPoint) (Variables|Default|GetendPoint) _alpha) true false)))))))

(fn ConstructionScript)

(fn SetFlattenedMesh
  (bind _chicken (Variables|Default|GetChicken))
  (switch int (Variables|Default|GetIAmType)
    (:0
      (Components|StaticMesh|SetStaticMesh _chicken "/Game/Meshes/flatchick.flatchick"))
    (:1
      (Components|StaticMesh|SetStaticMesh _chicken "/Game/Meshes/flatsheep.flatsheep"))
    (:2
      (Components|StaticMesh|SetStaticMesh _chicken "/Game/Meshes/flatsteer.flatsteer"))
    (:3
      (Components|StaticMesh|SetStaticMesh _chicken "/Game/Meshes/flathedgehog.flathedgehog"))))

(fn NormalSound
  (bind _normclucking (Variables|Default|GetnormClucking))
  (bind _normdeer (Variables|Default|GetnormDeer))
  (switch int (Variables|Default|GetIAmType)
    (:0
      ;[1 1 1] Chance to Cluck
      (if (>= (Math|Random|RandomIntegerinRange 0 10) 9)
        (Audio|Components|Audio|FadeIn _normclucking 0.0 1.0 0.0 :!class /Script/Engine.AudioComponent)
        (Audio|Components|Audio|FadeOut _normclucking 1.5 0.0 :!class /Script/Engine.AudioComponent)))
    (:1
      ;[1 1 1] Chance to Baaa
      (if (>= (Math|Random|RandomIntegerinRange 0 10) 9)
        (Audio|PlaySoundatLocation "/Game/Audio/baaa.baaa" (Transformation|GetWorldLocation (Variables|Default|GetChicken)) "0, 0, 0" 0.3 1.0 0.0 0 0 0)))
    (:2
      ;[1 1 1] Chance to Deer
      (if (>= (Math|Random|RandomIntegerinRange 0 10) 9)
        (Audio|Components|Audio|FadeIn _normdeer 0.0 1.0 0.0 :!class /Script/Engine.AudioComponent)
        (Audio|Components|Audio|FadeOut _normdeer 1.5 0.0 :!class /Script/Engine.AudioComponent)))
    (:3
      ;[1 1 1] Chance to Sonic
      (if (>= (Math|Random|RandomIntegerinRange 0 10) 9)
        (Audio|PlaySoundatLocation "/Game/Audio/tooSlowCue.tooSlowCue" (Transformation|GetWorldLocation (Variables|Default|GetChicken)) "0, 0, 0" 0.3 1.0 0.0 0 0 0)))))

(fn DeathSound
  (switch int (Variables|Default|GetIAmType)
    (:0
      ;[1 1 1] Chance to Cluck
      (Audio|PlaySoundatLocation "/Game/Audio/chickcluck.chickcluck" (Transformation|GetWorldLocation (Variables|Default|GetChicken)) "0, 0, 0" 1.0 1.0 0.0 0 0 0))
    (:1
      ;[1 1 1] Chance to Baaa
      (Audio|PlaySoundatLocation "/Game/Audio/baaa.baaa" (Transformation|GetWorldLocation (Variables|Default|GetChicken)) "0, 0, 0" 0.3 1.5 0.0 0 0 0))
    (:2
      ;[1 1 1] Chance to Deer
      (Audio|PlaySoundatLocation "/Game/Audio/deerSoundCue.deerSoundCue" (Transformation|GetWorldLocation (Variables|Default|GetChicken)) "0, 0, 0" 0.7 1.5 0.0 0 0 0))
    (:3
      ;[1 1 1] Chance to Sonic
      (Audio|PlaySoundatLocation "/Game/Audio/blehCue.blehCue" (Transformation|GetWorldLocation (Variables|Default|GetChicken)) "0, 0, 0" 0.7 1.0 0.0 0 0 0))))