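; Ground lane tile that spawns trees or traffic and destroys itself when the player overlaps its DespawnTrigger.
; On BeginPlay, EnemyType selects either trees at the spawn points gathered in the construction script, or a looping timer for cars, trucks or trains.
; Trains run on a fixed interval, while cars and trucks get a random interval rolled once and play a sound per spawn.
; A random SpawnSide fixes which end vehicles spawn from.
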(event OnComponentBeginOverlap(DespawnTrigger)
  (params (OverlappedComponent :type Primitive%20Component%20Object%20Reference) (OtherActor :type Actor%20Object%20Reference) (OtherComp :type Primitive%20Component%20Object%20Reference) (OtherBodyIndex :type Integer) (bFromSweep :type Boolean) (SweepResult :type Hit%20Result%20Structure%20%28by%20ref%29))
  ;[1 1 1] Destroy Old Ground
  (Utilities|Casting|CastToPlayerBP OtherActor)
  (Actor|DestroyActor))

(event Custom|TimeToSpawn
  ;[1 1 1] Figure Out What to Spawn
  (switch int (Variables|Default|GetEnemyType)
    (:1
      (CallFunction|SpawnCar)
      (Audio|PlaySoundatLocation "/Game/Audio/carCue.carCue" (Transformation|GetWorldLocation (Variables|Default|GetPlane)) "0, 0, 0" 1.0 1.0 0.0 0 0 0))
    (:2
      (CallFunction|SpawnTruck)
      (Audio|PlaySoundatLocation "/Game/Audio/truckCue.truckCue" (Transformation|GetWorldLocation (Variables|Default|GetPlane)) "0, 0, 0" 1.0 1.0 0.0 0 0 0))
    (:3
      (CallFunction|SpawnTrain))))

(event EventBeginPlay
  ;[1 1 1] Figure Out What to Spawn
  (Variables|Default|SetSpawnSide (Math|Random|RandomInteger 2))
  (Utilities|FlowControl|Delay 0.1)
  (if (== 0 (Variables|Default|GetEnemyType))
    (Utilities|FlowControl|Delay 0.2)
    (for _array_element (Variables|Default|GetTreeSpawns)
      (Game|SpawnActorfromClass "/Game/Blueprints/TreeBP.TreeBP_C" (Math|Transform|MakeTransform (Transformation|GetWorldLocation _array_element) "0, 0, 0" "1,1,1") "AlwaysSpawn" 0 0))
    (elif (== 3 (Variables|Default|GetEnemyType))
      (Utilities|Time|SetTimerbyEvent (delegate Custom|TimeToSpawn) 5.0 true)
      (else
        (Utilities|Time|SetTimerbyEvent (delegate Custom|TimeToSpawn) (Math|Random|RandomFloatinRange 1.5 4.0) true)))))

(fn ConstructionScript
  (bind _treespawns (Variables|Default|GetTreeSpawns))
  (Utilities|Array|SetArrayElem _treespawns 0 (Variables|Default|GetTreeSpawn))
  (Utilities|Array|SetArrayElem _treespawns 1 (Variables|Default|GetTreeSpawn2))
  (Utilities|Array|SetArrayElem _treespawns 2 (Variables|Default|GetTreeSpawn3))
  (Utilities|Array|SetArrayElem _treespawns 3 (Variables|Default|GetTreeSpawn4))
  (Utilities|Array|SetArrayElem _treespawns 4 (Variables|Default|GetTreeSpawn5))
  (Utilities|Array|SetArrayElem _treespawns 5 (Variables|Default|GetTreeSpawn6))
  (Utilities|Array|SetArrayElem _treespawns 6 (Variables|Default|GetTreeSpawn8))
  (Utilities|Array|SetArrayElem _treespawns 7 (Variables|Default|GetTreeSpawn9))
  (Utilities|Array|SetArrayElem _treespawns 8 (Variables|Default|GetTreeSpawn10)))

(fn SpawnCar
  (bind _enemyspawn2 (Variables|Default|GetEnemySpawn2))
  (bind _enemyspawn (Variables|Default|GetEnemySpawn))
  (switch int (Variables|Default|GetSpawnSide)
    (:0
      (Game|SpawnActorfromClass "/Game/Blueprints/carBP.carBP_C" (Math|Transform|MakeTransform (Transformation|GetWorldLocation _enemyspawn) (Transformation|GetWorldRotation _enemyspawn) "1,1,1") "AlwaysSpawn" 0 0))
    (:1
      (Game|SpawnActorfromClass "/Game/Blueprints/carBP.carBP_C" (Math|Transform|MakeTransform (Transformation|GetWorldLocation _enemyspawn2) (Transformation|GetWorldRotation _enemyspawn2) "1,1,1") "AlwaysSpawn" 0 0))))

(fn SpawnTruck
  (bind _enemyspawn (Variables|Default|GetEnemySpawn))
  (bind _enemyspawn2 (Variables|Default|GetEnemySpawn2))
  (switch int (Variables|Default|GetSpawnSide)
    (:0
      (Game|SpawnActorfromClass "/Game/Blueprints/truckBP.truckBP_C" (Math|Transform|MakeTransform (Transformation|GetWorldLocation _enemyspawn) (Transformation|GetWorldRotation _enemyspawn) "1,1,1") "AlwaysSpawn" 0 0))
    (:1
      (Game|SpawnActorfromClass "/Game/Blueprints/truckBP.truckBP_C" (Math|Transform|MakeTransform (Transformation|GetWorldLocation _enemyspawn2) (Transformation|GetWorldRotation _enemyspawn2) "1,1,1") "AlwaysSpawn" 0 0))))

(fn SpawnTrain
  (bind _enemyspawn2 (Variables|Default|GetEnemySpawn2))
  (bind _enemyspawn (Variables|Default|GetEnemySpawn))
  (switch int (Variables|Default|GetSpawnSide)
    (:0
      (Game|SpawnActorfromClass "/Game/Blueprints/trainBP.trainBP_C" (Math|Transform|MakeTransform (Transformation|GetWorldLocation _enemyspawn) (Transformation|GetWorldRotation _enemyspawn) "1,1,1") "AlwaysSpawn" 0 0))
    (:1
      (Game|SpawnActorfromClass "/Game/Blueprints/trainBP.trainBP_C" (Math|Transform|MakeTransform (Transformation|GetWorldLocation _enemyspawn2) (Transformation|GetWorldRotation _enemyspawn2) "1,1,1") "AlwaysSpawn" 0 0))))