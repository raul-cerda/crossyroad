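; A title Blueprint that animates a Wording component through a two-stage move when play begins.
; A first timeline lerps the wording from StartLoc to EndLoc.
; After a short pause, the old end becomes the new start, the target shifts along negative Y, and a second timeline carries the wording on to it.
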(event EventBeginPlay
  (bind _newtrack_0 (Timeline|MoveTitleOverTime PlayFromStart)
    (:Update
      (Transformation|SetWorldLocation (Variables|Default|Getwording) (Math|Vector|Lerp(Vector) (Variables|Default|GetstartLoc) (Variables|Default|GetendLoc) _newtrack_0) false false))
    (:Finished
      (Utilities|FlowControl|Delay 3.0)
      (Variables|Default|SetstartLoc (Variables|Default|GetendLoc))
      (Variables|Default|SetendLoc (+ "0,-500.000000, 0" (Variables|Default|GetstartLoc)))
      (bind _newtrack_0_2 (Timeline|Timeline_0 PlayFromStart)
        (:Update
          (Transformation|SetWorldLocation (Variables|Default|Getwording) (Math|Vector|Lerp(Vector) (Variables|Default|GetstartLoc) (Variables|Default|GetendLoc) _newtrack_0_2) false false))))))

(fn ConstructionScript)